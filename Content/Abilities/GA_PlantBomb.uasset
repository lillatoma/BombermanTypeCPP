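; GA_PlantBomb is a Gameplay Ability that plants a BP_Bomb at the owner actor's location and rotation.
; On activation it reads a float attribute from the owner's Ability System Component and only spawns the bomb when the value is above zero.
; After spawning it applies GE_BombReduced to the owner, and the ability ends immediately whether or not a bomb was placed.
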(event `self.K2_ActivateAbility`
  (bind _returnvalue_owneractor (break `GameplayAbilityActorInfo` (`self.GetActorInfo`)))
  (if (> (`.ReturnValue` (`AbilitySystemBlueprintLibrary.GetFloatAttributeFromAbilitySystemComponent` (`AbilitySystemBlueprintLibrary.GetAbilitySystemComponent` _returnvalue_owneractor) (struct :`AttributeName` "BombCount" :`Attribute` "/Script/BombermanTypeCPP.GAS_AttributeSet:BombCount" :`AttributeOwner` "Class'\"/Script/BombermanTypeCPP.GAS_AttributeSet\"'"))) 0.0)
    (`|SpawnActorFromClass` "/Game/BP_Bomb.BP_Bomb_C" (`KismetMathLibrary.MakeTransform` (.location (`Actor.GetTransform` _returnvalue_owneractor)) (.rotation (`Actor.GetTransform` _returnvalue_owneractor))) "Undefined" "OverrideRootScale" null null)
    (`self.BP_ApplyGameplayEffectToOwner` "/Game/Abilities/GE_BombReduced.GE_BombReduced_C")
    (`self.K2_EndAbility`)
    (else
      (`self.K2_EndAbility`))))